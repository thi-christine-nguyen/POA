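; BP_SecurityAgent is an enemy agent with a melee attack aimed at the top-down player character.
; MeleeAttack plays an attack montage, with a 2D sound once it starts.
; When the montage's notify begins, a sphere overlap at the Sphere component finds BP_TopDownCharacter pawns, draws a debug sphere and applies damage to each, instigated by the agent's controller.
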(event EventMeleeAttack
  (bind _sphere (Variables|Default|GetSphere))
  (bind _returnvalue (Transformation|GetWorldLocation _sphere))
  ;[1 1 1] Animation d'attaque
  (Animation|Montage|PlayMontage (Variables|Character|GetMesh) "/Game/SecurityAgent/Animations/MontageAttack.MontageAttack"
    (:then
      ;;[1 1 1] Points de vie
      (Audio|PlaySound2D "/Game/StoneDistraction/stone-dropping-6843.stone-dropping-6843" 0.5 1.0 0.0 0 0))
    (:OnNotifyBegin
      (bind _outactors (Collision|SphereOverlapActors _returnvalue (Variables|Combat|GetAttack%20Sphere%20Radius) (Utilities|Array|MakeArray "ObjectTypeQuery3") "/Game/TopDown/Blueprints/BP_TopDownCharacter.BP_TopDownCharacter_C" (Utilities|Array|MakeArray self)))
      (Rendering|Debug|DrawDebugSphere _returnvalue (Variables|Combat|GetAttack%20Sphere%20Radius) 12 "(R=0.583333,G=0.009772,B=0.000000,A=1.000000)" (Variables|DebugTools|GetSphere%20Duration))
      (for _array_element _outactors
        (Game|Damage|ApplyDamage _array_element (Variables|Combat|GetAttack%20Base%20Damage) (Pawn|GetController) self "/Script/Engine.DamageType")))))

(fn ConstructionScript)