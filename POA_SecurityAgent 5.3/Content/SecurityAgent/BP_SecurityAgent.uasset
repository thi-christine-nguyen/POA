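; Security agent AI that wanders to random nearby navigable points, pausing briefly, and reacts to pawns it detects.
; PawnSensing sightings start a chase with a one-time sprint, reset after a retriggerable lose-focus delay or on arrival.
; AIPerception stimuli from the top-down character make it run to the location and investigate before resuming patrol.
; Event-driven AIMoveTo replaces a behavior tree, with Walk, Run and Idle functions playing animations directly, the first two also setting speed.
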(event OnSeePawn(PawnSensing)
  (params (Pawn :type Pawn%20Object%20Reference))
  (Utilities|FlowControl|Sequence
    (:then_0
      (Utilities|FlowControl|DoOnce false
        (:Completed
          (CallFunction|Run))))
    (:then_1
      (AI|AIMoveTo self "0, 0, 0" Pawn 25.0 false
        (:then
          (Utilities|FlowControl|RetriggerableDelay (Variables|Default|GetDelayToLooseFocus)))
        (:OnSuccess
          _))
      (CallFunction|Walk)
      (CallFunction|CanSprintAgain)
      (CallFunction|MovetoRandomLocation))))

(event OnTargetPerceptionUpdated(AIPerception)
  (params (Actor :type Actor%20Object%20Reference) (Stimulus :type AI%20Stimulus%20Structure))
  (bind (_age _expirationage _strength _stimuluslocation _receiverlocation _tag _bsuccessfullysensed) (Utilities|Struct|BreakAIStimulus Stimulus))
  (Utilities|Casting|CastToBP_TopDownCharacter Actor)
  (if _bsuccessfullysensed
    (Variables|Default|SetInvestigating true)
    (CallFunction|Run)
    (AI|AIMoveTo self _stimuluslocation 0 5.0 false
      (:OnSuccess
        (CallFunction|Idle)
        (Utilities|FlowControl|Delay (Variables|Default|GetTimeOfInvestigation))
        (Variables|Default|SetInvestigating false)
        (CallFunction|Walk)
        (CallFunction|MovetoRandomLocation)))))

(event Custom|MoveToRandomLocation
  (bind _randomlocation (Class|NavigationSystemV1|GetRandomLocationinNavigableRadius (Transformation|GetActorLocation) 1e+03 0 0))
  (AI|AIMoveTo self _randomlocation 0 5.0 false
    (:OnSuccess
      (CallFunction|Idle)
      (Utilities|FlowControl|Delay (Math|Random|RandomFloatinRange 1.0 3.0))
      (CallFunction|Walk)
      (if (not (Variables|Default|GetInvestigating))
        (CallFunction|MovetoRandomLocation :!label _label)))
    (:OnFail
      (goto _label))))

(event Custom|CanSprintAgain
  (Utilities|FlowControl|DoOnce false) ; enters at Reset
)

(event EventBeginPlay
  (CallFunction|MovetoRandomLocation))

(fn ConstructionScript)

(fn Walk
  (Components|Animation|PlayAnimation (Variables|Character|GetMesh) "/Game/Characters/Mannequins/Animations/Manny/MM_Walk_Fwd.MM_Walk_Fwd" true)
  (Variables|/Script/Engine.CharacterMovementComponent|SetMaxWalkSpeed (Variables|Character|GetCharacterMovement) 1.5e+02))

(fn Run
  (Components|Animation|PlayAnimation (Variables|Character|GetMesh) "/Game/Characters/Mannequins/Animations/Manny/MM_Run_Fwd.MM_Run_Fwd" true)
  (Variables|/Script/Engine.CharacterMovementComponent|SetMaxWalkSpeed (Variables|Character|GetCharacterMovement) 4.5e+02))

(fn Idle
  (Components|Animation|PlayAnimation (Variables|Character|GetMesh) "/Game/Characters/Mannequins/Animations/Manny/MM_Idle.MM_Idle" true)
  (return))